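; Test actor that periodically grants experience to characters standing inside its Box volume.
; On BeginPlay, GiveExp starts a looping one-second timer that calls GiveExpToCharacter.
; Each tick of the timer finds overlapping PitCharacters and credits their PlayerState with a fixed amount through PitGameState's PlayerGainExperience, printing a debug string.
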(event Custom|GiveExp
  (Utilities|Time|SetTimerbyFunctionName 0 "GiveExpToCharacter" 1.0 true))

(event EventBeginPlay
  (CallFunction|GiveExp))

(event Collision|EventActorBeginOverlap
  (params (OtherActor :type Actor%20Object%20Reference)))

(event EventTick
  (params (DeltaSeconds :type Float%20%28single-precision%29)))

(fn ConstructionScript)

(fn GiveExptoCharacter
  (bind _aspit_game_state (Utilities|Casting|CastToPitGameState (Game|GetGameState)))
  (for _array_element (Collision|GetOverlappingActors (Variables|Default|GetBox) "/Script/ThePit.PitCharacter" :!class /Script/Engine.PrimitiveComponent)
    (bind _aspit_character (Utilities|Casting|CastToPitCharacter _array_element))
    (Class|PitGameState|PlayerGainExperience _aspit_game_state (Variables|/Script/Engine.Pawn|GetPlayerState _aspit_character) 33)
    (Development|PrintString "Shit can")))