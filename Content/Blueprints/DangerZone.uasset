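; DangerZone is a hazard volume actor that deals damage over time to PitCharacters standing inside its box.
; On BeginPlay it starts a looping one-second timer that calls DamageActorsInside by name.
; That function queries the box for overlapping PitCharacters, applies a small fixed damage to each through TakeDamage, and prints a message naming the hero hit.
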(event Custom|DangerZoneDamage
  (Utilities|Time|SetTimerbyFunctionName 0 "DamageActorsInside" 1.0 true))

(event EventBeginPlay
  (CallFunction|DangerZoneDamage))

(event Collision|EventActorBeginOverlap
  (params (OtherActor :type Actor%20Object%20Reference)))

(event EventTick
  (params (DeltaSeconds :type Float%20%28single-precision%29)))

(fn ConstructionScript)

(fn DamageActorsInside
  (for _array_element (Collision|GetOverlappingActors (Variables|Default|GetBox) "/Script/ThePit.PitCharacter" :!class /Script/Engine.PrimitiveComponent)
    (bind _aspit_character (Utilities|Casting|CastToPitCharacter _array_element))
    (Class|PitCharacter|TakeDamage _aspit_character 1.0 (Utilities|Struct|MakeDamageEvent))
    (Development|PrintString (Utilities|String|ToString(Text) (Utilities|Text|FormatText "{character} is taking damage" (Utilities|Text|ToText(String) (Variables|/Script/ThePit.PitCharacter|GetHeroName _aspit_character)))))))